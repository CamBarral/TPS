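; BP_FarmTile is a farm plot that grows a carrot through three mesh stages, with a countdown shown in 3D text.
; Tick, gated by IsSomethingPlanted, reads the player character's Seed and calls PlantCarrot for seed 0.
; PlantCarrot swaps runtime-added static mesh components after each of two GrowTime waits.
; GrowTime is a reusable one-second Delay loop that updates the text until zero.
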(event Custom|PlantCarrot
  (bind _relativetransformlocation (Variables|Default|GetRelativeTransformLocation))
  (bind _returnvalue (AddComponent|AddStaticMeshComponent false (Math|Transform|MakeTransform _relativetransformlocation "0, 0, 0" "1,1,1")))
  (Utilities|GrowTime (Variables|Default|GetCarrotGrowTime)
    (:Out
      (Components|DestroyComponent _returnvalue)
      (bind _returnvalue_2 (AddComponent|AddStaticMeshComponent false (Math|Transform|MakeTransform _relativetransformlocation "0, 0, 0" "1,1,1")))
      (Utilities|GrowTime (Variables|Default|GetCarrotGrowTime)
        (:Out
          (Components|DestroyComponent _returnvalue_2)
          (AddComponent|AddStaticMeshComponent false (Math|Transform|MakeTransform _relativetransformlocation "0, 0, 0" "1,1,1")))))))

(event EventBeginPlay
  (Class|Text3DComponent|SetText (Variables|Default|GetText3D) (Variables|Default|GetValue)))

(event EventTick
  (params (DeltaSeconds :type Float%20%28single-precision%29))
  (if (Variables|Default|GetIsSomethingPlanted?)
    (bind _asthird_person_character (Utilities|Casting|CastToThirdPersonCharacter (Game|GetPlayerCharacter 0)))
    (switch int (Variables|/Game/ThirdPersonBP/Blueprints/ThirdPersonCharacter.ThirdPersonCharacter_C|GetSeed _asthird_person_character)
      (:0
        (CallFunction|PlantCarrot)
        (Variables|Default|SetIsSomethingPlanted? true)))))

(fn ConstructionScript)